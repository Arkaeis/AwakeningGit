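; Behavior tree service that drives enemy aggro by writing the AI state (Idle, Combat, Searching, Panic) to the Blackboard.
; Each tick, a view-angle check and line trace set Combat when the player is visible.
; A spawned TargetPoint memory marker stores the last seen location, switching to Searching when sight fails, or Idle without a marker.
; The enemy's Blowtorched event clears the target and sets Panic; a debug option draws the marker.
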(event `self.ReceiveActivationAI`
  (params (OwnerController :type "AIController Object Reference") (ControlledPawn :type "Pawn Object Reference"))
  ;[1 1 1] On AI Start, set to state to Idle
  (`BTFunctionLibrary.SetBlackboardValueAsEnum` (`self.State`) (enumliteral `/Game/Logic/Blueprints/AI/AIState` "NewEnumerator0"))
  ;[1 1 1] When Enemy is blowtorched, set state to Panic
  (bind _asenemy_bp (cast `/Game/Logic/Blueprints/AI/EnemyBP` ControlledPawn))
  (add `/Game/Logic/Blueprints/AI/EnemyBP.Blowtorched` _asenemy_bp (delegate `ChangeStateToPanic`)))

(event `ChangeStateToPanic`
  ;[1 1 1] When Enemy is blowtorched, set state to Panic
  (`BTFunctionLibrary.SetBlackboardValueAsObject` (`self.TargetActor`))
  (`BTFunctionLibrary.SetBlackboardValueAsEnum` (`self.State`) (enumliteral `/Game/Logic/Blueprints/AI/AIState` "NewEnumerator2")))

(event `self.ReceiveTickAI`
  (params (OwnerController :type "AIController Object Reference") (ControlledPawn :type "Pawn Object Reference") (DeltaSeconds :type "Float (single-precision)"))
  (bind _returnvalue (`GameplayStatics.GetPlayerCharacter` 0))
  (bind _returnvalue_2 (`Actor.K2_GetActorLocation` ControlledPawn))
  (bind _returnvalue_3 (`BTFunctionLibrary.GetBlackboardValueAsActor` (`self.MemoryMarker`)))
  (bind _returnvalue_4 (`BTFunctionLibrary.GetBlackboardValueAsActor` (`self.MemoryMarker`)))
  (bind _returnvalue_5 (`Actor.K2_GetActorLocation` (`GameplayStatics.GetPlayerCharacter` 0)))
  (`|ExecutionSequence`
    (:`then_0`
      ;[1 1 1] If player is within vision radius, state is Combat
      (if (< (`KismetMathLibrary.DegAcos` (`KismetMathLibrary.Dot_VectorVector` (`KismetMathLibrary.Normal` (- _returnvalue_5 _returnvalue_2)) (`Actor.GetActorForwardVector` ControlledPawn))) (`self.EnemyVisionRadius`))
        (bind _ascharacter (cast `Character` ControlledPawn))
        (bind _outhit (`KismetSystemLibrary.LineTraceSingle` _returnvalue_2 _returnvalue_5 "TraceTypeQuery2" false (`|MakeArray` (`ActorComponent.GetOwner` (`Character.CapsuleComponent` _ascharacter)))))
        (bind _ascharacter_2 (cast `Character` (`.HitActor` (`GameplayStatics.BreakHitResult` _outhit)))
          (:`then`
            (if (== _ascharacter_2 (`GameplayStatics.GetPlayerCharacter` 0))
              (`BTFunctionLibrary.SetBlackboardValueAsObject` (`self.TargetActor`) _returnvalue)
              (if (!= _returnvalue_3 null)
                (`Actor.K2_SetActorLocation` _returnvalue_3 (`Actor.K2_GetActorLocation` _returnvalue) false false)
                (else
                  (bind _returnvalue_6 (`|SpawnActorFromClass` "/Script/Engine.TargetPoint" (`Actor.GetTransform` _returnvalue) "AlwaysSpawn" "OverrideRootScale"))))
              (`BTFunctionLibrary.SetBlackboardValueAsObject` (`self.MemoryMarker`) _returnvalue_6)
              (`BTFunctionLibrary.SetBlackboardValueAsEnum` (`self.State`) (enumliteral `/Game/Logic/Blueprints/AI/AIState` "NewEnumerator1"))
              (else
                ;[1 1 1] If AI previously sighted player, state is Searching, otherwise set to Idle
                (if (!= (`BTFunctionLibrary.GetBlackboardValueAsActor` (`self.MemoryMarker`)) null) :!label _label
                  (`BTFunctionLibrary.SetBlackboardValueAsEnum` (`self.State`) (enumliteral `/Game/Logic/Blueprints/AI/AIState` "NewEnumerator3"))
                  (else
                    (`BTFunctionLibrary.SetBlackboardValueAsObject` (`self.TargetActor`))
                    (`BTFunctionLibrary.SetBlackboardValueAsEnum` (`self.State`) (enumliteral `/Game/Logic/Blueprints/AI/AIState` "NewEnumerator0")))))))
          (:`CastFailed`
            (goto _label)))
        (else
          (goto _label))))
    (:`then_1`
      ;[1 1 1] If in Debug, show AI movement target
      (if (`self.Debug`)
        (if (!= _returnvalue_4 null)
          (`KismetSystemLibrary.DrawDebugSphere` (`Actor.K2_GetActorLocation` _returnvalue_4) 50.0 12 (struct :`R` 0.628503 :`G` 0.197308 :`B` 1.0 :`A` 1.0) 1.0))))))