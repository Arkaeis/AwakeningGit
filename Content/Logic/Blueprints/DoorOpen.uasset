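; DoorOpen is a sliding door that the player toggles with Use, gated by a required glyph.
; Its TriggerBox enables player input on overlap and disables it on exit.
; On Use, if the PlayerBP's CurrentGlyph matches RequiredGlyph, a FlipFlop alternately plays and reverses the DoorSlide timeline, which lerps the door between DoorStart and DoorEnd.
; A DoorGlyphLibrary comparison loop is unwired, and CheckOpen is empty.
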(event `self.TriggerBox.OnComponentBeginOverlap`
  (params (OverlappedComponent :type "PrimitiveComponent Object Reference") (OtherActor :type "Actor Object Reference") (OtherComp :type "PrimitiveComponent Object Reference") (OtherBodyIndex :type Integer) (bFromSweep :type Boolean) (SweepResult :type "HitResult Structure (by ref)"))
  ;[1 1 1] Door Input
  (`self.EnableInput` (`GameplayStatics.GetPlayerController` 0)))

(event `self.TriggerBox.OnComponentEndOverlap`
  (params (OverlappedComponent :type "PrimitiveComponent Object Reference") (OtherActor :type "Actor Object Reference") (OtherComp :type "PrimitiveComponent Object Reference") (OtherBodyIndex :type Integer))
  ;[1 1 1] Door Input
  (`self.DisableInput` (`GameplayStatics.GetPlayerController` 0)))

(event `InputAction|Use`
  (params (Key :type "Key Structure" :default "AnyKey"))
  ;[1 1 1] Open/Close Door
  (:`Pressed`
    (bind _asplayer_bp (cast `/Game/Logic/Blueprints/Player/PlayerBP` (`GameplayStatics.GetPlayerCharacter` 0)))
    (if (== (`/Game/Logic/Blueprints/Player/PlayerBP.CurrentGlyph` _asplayer_bp) (`self.RequiredGlyph`))
      (set `self.CanOpenDoor?` true)
      (if (`self.CanOpenDoor?`)
        (`/Engine/EditorBlueprintResources/StandardMacros.FlipFlop`
          (:`A`
            (bind (_direction _doortransform) (`Timeline|Door Slide` :!label _label)
              (:`Update`
                (`SceneComponent.K2_SetRelativeLocation` (`self.Door`) (`KismetMathLibrary.VLerp` (`self.DoorStart`) (`self.DoorEnd`) _doortransform) false false))))
          (:`B`
            (goto _label :!via `Reverse`)))))))

(fn `CheckOpen`)

(fn `UserConstructionScript`)