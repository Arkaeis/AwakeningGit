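; Actor for one glyph slot on a door puzzle, showing its glyph through a DoorGlyphSlotUI widget component.
; On BeginPlay it pushes its GlyphIndex into the widget's CurrentGlyph.
; ChangeGlyph pushes the current index to the widget again, then calls CheckOpen on the parent DoorOpen actor so the door can re-evaluate.
; The index itself is not modified here.
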(event `self.ReceiveBeginPlay`
  (bind _asdoor_glyph_slot_ui (cast `/Game/Logic/Blueprints/UI/DoorGlyphSlotUI` (`WidgetComponent.GetUserWidgetObject` (`self.GlyphSlot`))))
  (set `/Game/Logic/Blueprints/UI/DoorGlyphSlotUI.CurrentGlyph` (`self.GlyphIndex`) _asdoor_glyph_slot_ui))

(fn `ChangeGlyph`
  (bind _asdoor_glyph_slot_ui (cast `/Game/Logic/Blueprints/UI/DoorGlyphSlotUI` (`WidgetComponent.GetUserWidgetObject` (`self.GlyphSlot`))))
  (set `/Game/Logic/Blueprints/UI/DoorGlyphSlotUI.CurrentGlyph` (`self.GlyphIndex`) _asdoor_glyph_slot_ui)
  (bind _asdoor_open (cast `/Game/Logic/Blueprints/DoorOpen` (`self.GetParentActor`)))
  (`/Game/Logic/Blueprints/DoorOpen.CheckOpen` _asdoor_open))

(fn `UserConstructionScript`)