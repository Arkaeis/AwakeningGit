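; Water obelisk Blueprint that reveals a staircase by sliding its Cover component aside when the player interacts with it.
; The first overlap by the player character, gated by DoOnce, stores an end location offset by TravelDistanceX and plays a timeline.
; Each update lerps the Cover's relative location from its current position toward that end using the DoorOpenRate track, so movement compounds rather than interpolating from a fixed start.
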(event `self.ReceiveActorBeginOverlap`
  (params (OtherActor :type "Actor Object Reference"))
  (bind _cover (`self.Cover`))
  (bind _returnvalue_location (`KismetMathLibrary.BreakTransform` (`SceneComponent.GetRelativeTransform` _cover)))
  ;[1 1 1] (vi) Interacting with Obelisk reveals staircase.
  (if (== OtherActor (`GameplayStatics.GetPlayerCharacter` 0))
    (`/Engine/EditorBlueprintResources/StandardMacros.DoOnce` false
      (:`Completed`
        (bind _output_get (set `self.DoorEnd` (+ _returnvalue_location (`self.TravelDistanceX`))))
        (bind (_direction _dooropenrate) (`Timeline|Timeline_0`)
          (:`Update`
            (`SceneComponent.K2_SetRelativeLocation` _cover (`KismetMathLibrary.VLerp` _returnvalue_location _output_get _dooropenrate) false false)))))))

(fn `UserConstructionScript`)